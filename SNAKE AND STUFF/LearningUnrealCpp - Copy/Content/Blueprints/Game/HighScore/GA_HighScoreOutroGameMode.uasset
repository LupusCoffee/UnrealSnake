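; Game mode for the high-score outro screen shown at the end of the snake game.
; On BeginPlay it shows the mouse cursor and reads the highest score and winning player name from the SnakeGameInstance.
; It then creates the W_HighScoreOutro widget, adds it to the viewport and passes both values to it for display.
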(event `self.ReceiveBeginPlay`
  (`|ExecutionSequence`
    (:`then_0`
      (set `PlayerController.bShowMouseCursor` true (`GameplayStatics.GetPlayerController` 0)))
    (:`then_1`
      (bind _assnake_game_instance (cast `SnakeGameInstance` (`GameplayStatics.GetGameInstance`)))
      (bind _returnvalue (`SnakeGameInstance.GetHighestScore` _assnake_game_instance))
      (bind _returnvalue_2 (`SnakeGameInstance.GetWinningPlayerName` _assnake_game_instance)))
    (:`then_2`
      (bind _returnvalue_3 (`|CreateWidget` "/Game/Blueprints/Widgets/W_HighScoreOutro.W_HighScoreOutro_C"))
      (`UserWidget.AddToViewport` _returnvalue_3 0)
      (`HighScoreOutroWidget.SetHighScore` _returnvalue_3 _returnvalue)
      (`HighScoreOutroWidget.SetWinningPlayer` _returnvalue_3 _returnvalue_2))))

(fn `UserConstructionScript`)